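; Game mode for the main menu that shows the mouse cursor, resets ignored move input and sets up save access on BeginPlay.
; It creates a fresh MySaveGame object, whose slot name and user index identify the slot to read.
; LoadProgress loads that slot and returns progress, scores and stars, stopping if the cast to MySaveGame fails.
; An unconnected debug node can delete the saved slot.
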(event EventBeginPlay
  (bind _returnvalue (Game|GetPlayerController 0))
  (Variables|/Script/Engine.PlayerController|SetbShowMouseCursor _returnvalue true)
  (Input|ResetIgnoreMoveInput _returnvalue)
  (bind _returnvalue_2 (SaveGame|CreateSaveGameObject "/Game/Blueprints/MySaveGame.MySaveGame_C"))
  (bind _output_get (Variables|Private|SetsaveGame _returnvalue_2)))

(fn ConstructionScript)

(fn LoadProgress
  (bind _savegame (Variables|Private|GetsaveGame))
  (bind _returnvalue (SaveGame|LoadGamefromSlot (Variables|/Game/Blueprints/MySaveGame.MySaveGame_C|GetsaveSlotName _savegame) (Variables|/Game/Blueprints/MySaveGame.MySaveGame_C|GetUserIndex _savegame)))
  (bind _asmy_save_game (Utilities|Casting|CastToMySaveGame _returnvalue))
  (return (Variables|/Game/Blueprints/MySaveGame.MySaveGame_C|Getprogress _asmy_save_game) (Variables|/Game/Blueprints/MySaveGame.MySaveGame_C|Getscores _asmy_save_game) (Variables|/Game/Blueprints/MySaveGame.MySaveGame_C|Getstars _asmy_save_game)))