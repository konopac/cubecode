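; HUD Blueprint that creates the main menu widget and adds it to the viewport on BeginPlay.
; It also defines CreateLevelSelection to build numbered level buttons, starting a new Box widget in the menu's LevelButtons container every five buttons.
; Each button's overlay is assigned to the current Box's overlay variable rather than added as a child.
; The CreateLevelSelection call is disconnected, so the level grid is never built.
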(event EventBeginPlay
  (bind _returnvalue (UserInterface|CreateWidget "/Game/Blueprints/MainMenu/MainMenuWidget.MainMenuWidget_C"))
  (UserInterface|Viewport|AddtoViewport _returnvalue 0))

(fn ConstructionScript)

(fn CreateLevelSelection
  (params (parent :type Main%20Menu%20Widget%20Object%20Reference))
  (for (_array_element _array_index) (Utilities|Array|MakeArray 1 2 3 4 5 6 7 8 9 10 11 12 13 14 15 16 17 18 19 20)
    ;[1 1 1] 5 buttons are packed in one horizontal box
    (if (== (Math|Integer|%(Integer) _array_index 5) 0)
      (bind _returnvalue (UserInterface|CreateWidget "/Game/Blueprints/MainMenu/Box.Box_C"))
      (bind _output_get (Variables|Default|SetcurrentHorizontalBox _returnvalue))
      (Widget|Panel|AddChild (Variables|/Game/Blueprints/MainMenu/MainMenuWidget.MainMenuWidget_C|GetLevelButtons parent) _output_get))
    (bind _returnvalue_2 (UserInterface|CreateWidget "/Game/Blueprints/MainMenu/LevelButton.LevelButton_C"))
    (Rendering|Components|TextRender|SetText (Variables|/Game/Blueprints/MainMenu/LevelButton.LevelButton_C|GetText _returnvalue_2) (Utilities|Text|ToText(Integer) _array_element))
    (bind _asbox (Utilities|Casting|CastToBox (Variables|Default|GetcurrentHorizontalBox)))
    (Variables|/Game/Blueprints/MainMenu/Box.Box_C|SetOverlay1 _asbox (Variables|/Game/Blueprints/MainMenu/LevelButton.LevelButton_C|GetOverlay_0 _returnvalue_2))))