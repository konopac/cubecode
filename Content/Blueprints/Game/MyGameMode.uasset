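; Game mode for a cube-based level that runs setup, win, fail and replay, and tracks time, stars and score.
; On start it records breakable cubes, randomly lengthens the level, spawns the DarkCube at the StartCube and creates widgets.
; Expansion shifts cubes beyond the ExpandingCube line and fills the gap with copies.
; Failure or replay resets cubes and UI, respawns missing breakables, re-expands and replaces the DarkCube.
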(event Custom|Failed
  ;[1 1 1] Pause game
  (Variables|Public|SetgameOver true)
  (bind _myplayercontroller (Helper|GetMyPlayerController))
  (Default|PauseMovement _myplayercontroller)
  (Default|Failed (Variables|Public|GetdarkCube))
  (Utilities|FlowControl|Delay 1.0)
  ;[1 1 1] Show failed widget
  (bind _myhud (Helper|GetMyHUD))
  (UserInterface|Viewport|AddtoViewport (Variables|/Game/Blueprints/Game/MyHUD.MyHUD_C|GetFailedWidget _myhud) 0)
  (bind _percent (Timeline|FailedWidgetTimeline PlayFromStart)
    (:Update
      (Widget|SetRenderOpacity (Variables|/Game/Blueprints/Game/MyHUD.MyHUD_C|GetFailedWidget _myhud) _percent))
    (:Finished
      (Widget|RemovefromParent (Variables|/Game/Blueprints/Game/MyHUD.MyHUD_C|GetFailedWidget _myhud))
      (Public|ResetAllCubes))))

(event Custom|Victory
  ;[1 1 1] Pause game and calculate score
  (Variables|Public|SetgameOver true)
  (bind _myplayercontroller (Helper|GetMyPlayerController))
  (Default|PauseMovement _myplayercontroller)
  (Private|CalculateScore)
  (Default|Victory (Variables|Public|GetdarkCube))
  (Utilities|FlowControl|Delay 1.0)
  ;[1 1 1] Show victory widget
  (bind _myhud (Helper|GetMyHUD))
  (UserInterface|Viewport|AddtoViewport (Variables|/Game/Blueprints/Game/MyHUD.MyHUD_C|GetVictoryWidget _myhud) 0)
  (bind _percent (Timeline|VictoryWidgetTimeline PlayFromStart)
    (:Update
      (Widget|SetRenderOpacity (Variables|/Game/Blueprints/Game/MyHUD.MyHUD_C|GetVictoryWidget _myhud) _percent))))

(event Custom|Replay
  (Public|ResetAllCubes)
  (bind _myhud (Helper|GetMyHUD))
  (Widget|RemovefromParent (Variables|/Game/Blueprints/Game/MyHUD.MyHUD_C|GetVictoryWidget _myhud)))

(event EventBeginPlay
  (Private|StoreBreakableCubes)
  (Private|ExpandCubes)
  (Private|SpawnDarkCube)
  (Private|CreateandShowWidgets))

(fn ConstructionScript)

(fn SpawnDarkCube
  (bind _outactors (Actor|GetAllActorsOfClass "/Game/Blueprints/Game/Cubes/StartCube.StartCube_C"))
  (bind _returnvalue (Game|SpawnActorfromClass "/Game/Blueprints/Game/Cubes/DarkCube.DarkCube_C" (Math|Transform|MakeTransform (+ (.location (Transformation|GetWorldTransform (Variables|/Game/Blueprints/Game/Cubes/StartCube.StartCube_C|GetCube (Utilities|Array|Get(acopy) _outactors)))) "0,0.000000,100.000000") (.rotation (Transformation|GetWorldTransform (Variables|/Game/Blueprints/Game/Cubes/StartCube.StartCube_C|GetCube (Utilities|Array|Get(acopy) _outactors)))) (.scale (Transformation|GetWorldTransform (Variables|/Game/Blueprints/Game/Cubes/StartCube.StartCube_C|GetCube (Utilities|Array|Get(acopy) _outactors))))) "Undefined" 0 0))
  (Variables|Public|SetdarkCube _returnvalue))

(fn GetExpandingDirectionandLocation
  (bind _outactors (Actor|GetAllActorsOfClass "/Game/Blueprints/Game/Cubes/ExpandingCube.ExpandingCube_C"))
  (if (== (.x (Transformation|GetActorLocation (Utilities|Array|Get(acopy) _outactors))) (.x (Transformation|GetActorLocation (Utilities|Array|Get(acopy) _outactors 1))))
    (return (Math|Vector|MakeVector (.x (Transformation|GetActorLocation (Utilities|Array|Get(acopy) _outactors))) 0.0 0.0) (== (.x (Transformation|GetActorLocation (Utilities|Array|Get(acopy) _outactors))) (.x (Transformation|GetActorLocation (Utilities|Array|Get(acopy) _outactors 1)))))
    (elif (== (.y (Transformation|GetActorLocation (Utilities|Array|Get(acopy) _outactors))) (.y (Transformation|GetActorLocation (Utilities|Array|Get(acopy) _outactors 1))))
      (return (Math|Vector|MakeVector 0.0 (.y (Transformation|GetActorLocation (Utilities|Array|Get(acopy) _outactors 1))) 0.0) (== (.x (Transformation|GetActorLocation (Utilities|Array|Get(acopy) _outactors))) (.x (Transformation|GetActorLocation (Utilities|Array|Get(acopy) _outactors 1))))))))

(fn MoveAllCubes
  (params (direction%20and%20distance :type Vector) (start%20location :type Vector) (x%20direction :type Boolean))
  (bind _outactors (Actor|GetAllActorswithInterface "/Game/Blueprints/Game/Cubes/Cube.Cube_C"))
  (for _array_element _outactors
    (if x%20direction
      (if (> (.x (Transformation|GetActorLocation _array_element)) (.x start%20location))
        (Transformation|SetActorLocation _array_element (+ (Transformation|GetActorLocation _array_element) direction%20and%20distance) false false :!label _label))
      (elif (> (.y (Transformation|GetActorLocation _array_element)) (.y start%20location))
        (goto _label)))))

(fn ReplicateExpandingCubes
  (params (direction :type Vector) (start%20location :type Vector) (x%20direction :type Boolean))
  (bind _outactors (Actor|GetAllActorsOfClass "/Game/Blueprints/Game/Cubes/ExpandingCube.ExpandingCube_C"))
  (for _array_element _outactors
    (if x%20direction
      (if (== (.x (Transformation|GetActorLocation _array_element)) (.x start%20location))
        (while (< (LocalVariables|Getcounter) (Variables|Private|Getexpand))
          (bind _returnvalue (Game|SpawnActorfromClass "/Game/Blueprints/Game/Cubes/ExpandingCube.ExpandingCube_C" (Math|Transform|MakeTransform (+ (* (Math|Vector|MakeVector 1e+02 0.0 0.0) (+ (LocalVariables|Getcounter) 1)) (Transformation|GetActorLocation _array_element)) "0, 0, 0" "1,1,1") "Undefined" 0 0))
          (Variables|/Game/Blueprints/Game/Cubes/ExpandingCube.ExpandingCube_C|Setoriginal _returnvalue false)
          (bind _result (Math|Integer|IncrementInt (LocalVariables|Getcounter))
            (:%20%20
              (LocalVariables|Setcounter _result))))
        (LocalVariables|Setcounter 0 :!label _label))
      (elif (== (.y (Transformation|GetActorLocation _array_element)) (.y start%20location))
        (while (< (LocalVariables|Getcounter) (Variables|Private|Getexpand))
          (bind _returnvalue_2 (Game|SpawnActorfromClass "/Game/Blueprints/Game/Cubes/ExpandingCube.ExpandingCube_C" (Math|Transform|MakeTransform (+ (* (Math|Vector|MakeVector 0.0 1e+02 0.0) (+ (LocalVariables|Getcounter) 1)) (Transformation|GetActorLocation _array_element)) "0, 0, 0" "1,1,1") "Undefined" 0 0))
          (Variables|/Game/Blueprints/Game/Cubes/ExpandingCube.ExpandingCube_C|Setoriginal _returnvalue_2 false)
          (bind _result_2 (Math|Integer|IncrementInt (LocalVariables|Getcounter))
            (:%20%20
              (LocalVariables|Setcounter _result_2))))
        (goto _label)))))

(fn ExpandCubes
  (bind (_result _x_direction) (Private|GetExpandingDirectionandLocation))
  (bind _output_get (Variables|Private|Setexpand (Math|Random|RandomIntegerinRange 0 5)))
  (Private|MoveAllCubes (Math|Vector|MakeVector (Math|Float|Absolute(Float) (.x (* (* (Math|Vector|Normalize _result) _output_get) "100.000000,100.000000, 0"))) (Math|Float|Absolute(Float) (.y (* (* (Math|Vector|Normalize _result) _output_get) "100.000000,100.000000, 0"))) (Math|Float|Absolute(Float) (.z (* (* (Math|Vector|Normalize _result) _output_get) "100.000000,100.000000, 0")))) _result _x_direction)
  (Private|ReplicateExpandingCubes (Math|Vector|MakeVector (Math|Float|Absolute(Float) (.x (* (* (Math|Vector|Normalize _result) _output_get) "100.000000,100.000000, 0"))) (Math|Float|Absolute(Float) (.y (* (* (Math|Vector|Normalize _result) _output_get) "100.000000,100.000000, 0"))) (Math|Float|Absolute(Float) (.z (* (* (Math|Vector|Normalize _result) _output_get) "100.000000,100.000000, 0")))) _result _x_direction))

(fn IncrementTime
  (bind _output_get (Variables|Public|SetcurrentTime (+ (Variables|Public|GetcurrentTime) 1)))
  ;[1 1 1] Update Time in HUD
  (bind _myhud (Helper|GetMyHUD))
  (Default|UpdateTime (Variables|/Game/Blueprints/Game/MyHUD.MyHUD_C|GetGameWidget _myhud) _output_get))

(fn GetMyHUD
  (bind _asmy_hud (Utilities|Casting|CastToMyHUD (HUD|GetHUD (Game|GetPlayerController 0))))
  (return _asmy_hud))

(fn IncrementStars
  (Variables|Public|SetcurrentStars (+ (Variables|Public|GetcurrentStars) 1)))

(fn CalculateScore
  (bind _output_get (Variables|Public|SetcurrentScore (- (+ (LocalVariables|GetmaxScore) (* (Variables|Public|GetcurrentStars) (LocalVariables|GetstarsWeight))) (* (* (Variables|Public|GetcurrentTime) (LocalVariables|GettimeWeight)) (* (Variables|Public|GetcurrentLines) (LocalVariables|GetlinesWight))))))
  (return _output_get))

(fn GetMyPlayerController
  (bind _asmy_player (Utilities|Casting|CastToMyPlayer (Game|GetPlayerController 0)))
  (return _asmy_player))

(fn ResetAllCubes
  (bind _outactors (Actor|GetAllActorsOfClass "/Game/Blueprints/Game/Cubes/ResetableCube.ResetableCube_C"))
  (for _array_element _outactors
    (Default|CustomReset _array_element))
  ;[1 1 1] Respawn broken cubes
  (for _array_element_2 (Variables|Private|GetbreakableCubeLocations)
    (LocalVariables|Setfound false)
    (bind _outactors_2 (Actor|GetAllActorsOfClass "/Game/Blueprints/Game/Cubes/BrokenCube.BrokenCube_C"))
    (for _array_element_3 _outactors_2
      (if (Math|Vector|Equal(Vector) (Transformation|GetActorLocation _array_element_3) (.location _array_element_2) 0.1)
        (LocalVariables|Setfound true)))
    (if (not (LocalVariables|Getfound))
      (Game|SpawnActorfromClass "/Game/Blueprints/Game/Cubes/BrokenCube.BrokenCube_C" (Math|Transform|MakeTransform (.location _array_element_2) (.rotation _array_element_2) (.scale _array_element_2)) "Undefined" 0 0)))
  (CallFunction|ResetUI)
  (Private|ExpandCubes)
  (Actor|DestroyActor (Variables|Public|GetdarkCube))
  (Private|SpawnDarkCube)
  (bind _myplayercontroller (Helper|GetMyPlayerController))
  (Default|SetDarkCube _myplayercontroller)
  (Default|ResumeMovement _myplayercontroller)
  (Variables|Public|SetgameOver false))

(fn CreateandShowWidgets
  (bind _myhud (Helper|GetMyHUD))
  (bind _returnvalue (UserInterface|CreateWidget "/Game/Blueprints/Game/Widgets/GameWidget.GameWidget_C"))
  (bind _output_get (Variables|/Game/Blueprints/Game/MyHUD.MyHUD_C|SetGameWidget _myhud _returnvalue))
  (UserInterface|Viewport|AddtoViewport _output_get 0)
  (bind _returnvalue_2 (UserInterface|CreateWidget "/Game/Blueprints/Game/Widgets/VictoryWidget.VictoryWidget_C"))
  (Variables|/Game/Blueprints/Game/MyHUD.MyHUD_C|SetVictoryWidget _myhud _returnvalue_2)
  (bind _returnvalue_3 (UserInterface|CreateWidget "/Game/Blueprints/Game/Widgets/FailedWidget.FailedWidget_C"))
  (Variables|/Game/Blueprints/Game/MyHUD.MyHUD_C|SetFailedWidget _myhud _returnvalue_3))

(fn StoreBreakableCubes
  (bind _outactors (Actor|GetAllActorsOfClass "/Game/Blueprints/Game/Cubes/BrokenCube.BrokenCube_C"))
  (for _array_element _outactors
    (Utilities|Array|Add (Variables|Private|GetbreakableCubeLocations) (Transformation|GetActorTransform _array_element))))

(fn ResetUI
  (Variables|Public|SetcurrentStars 0)
  (bind _output_get (Variables|Public|SetcurrentTime 0))
  (Variables|Public|SetcurrentLines 0)
  (Variables|Public|SetcurrentScore 0)
  (bind _myhud (Helper|GetMyHUD))
  (Default|UpdateTime (Variables|/Game/Blueprints/Game/MyHUD.MyHUD_C|GetGameWidget _myhud) _output_get))