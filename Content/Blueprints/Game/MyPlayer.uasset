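; Player controller for a cube-rolling game that turns directional input into 90-degree rolls of the game mode's DarkCube.
; A timeline rotates the cube around its calculated pivot, ignoring new rolls until it finishes.
; Each roll increments game time, notifies action cubes on leaving and landing, and fails the game when no cube lies underneath.
; The UI toggle switches between game-only and game-and-UI input until game over.
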(event EventBeginPlay
  (Public|SetDarkCube)
  (Public|PauseMovement))

(event Input|ActionEvents|InputActionRollEast
  (params (Key :type Key%20Structure))
  ;[1 1 1] Roll Movement
  (:Pressed
    (Variables|Default|Seteast 1)
    (if (not (Variables|/Game/Blueprints/Game/Cubes/DarkCube.DarkCube_C|GetisRolling (Variables|Default|GetdarkCube)))
      (Private|StartRoll)
      (bind _percent (Timeline|rollTimeline PlayFromStart)
        (:Update
          (Private|Roll _percent))
        (:Finished
          (Private|EndRoll))))))

(event Input|ActionEvents|InputActionRollNorth
  (params (Key :type Key%20Structure))
  ;[1 1 1] Roll Movement
  (:Pressed
    (Variables|Default|Setnorth 1)
    (if (not (Variables|/Game/Blueprints/Game/Cubes/DarkCube.DarkCube_C|GetisRolling (Variables|Default|GetdarkCube)))
      (Private|StartRoll)
      (bind _percent (Timeline|rollTimeline PlayFromStart)
        (:Update
          (Private|Roll _percent))
        (:Finished
          (Private|EndRoll))))))

(event Input|ActionEvents|InputActionRollSouth
  (params (Key :type Key%20Structure))
  ;[1 1 1] Roll Movement
  (:Pressed
    (Variables|Default|Setnorth -1)
    (if (not (Variables|/Game/Blueprints/Game/Cubes/DarkCube.DarkCube_C|GetisRolling (Variables|Default|GetdarkCube)))
      (Private|StartRoll)
      (bind _percent (Timeline|rollTimeline PlayFromStart)
        (:Update
          (Private|Roll _percent))
        (:Finished
          (Private|EndRoll))))))

(event Input|ActionEvents|InputActionRollWest
  (params (Key :type Key%20Structure))
  ;[1 1 1] Roll Movement
  (:Pressed
    (Variables|Default|Seteast -1)
    (if (not (Variables|/Game/Blueprints/Game/Cubes/DarkCube.DarkCube_C|GetisRolling (Variables|Default|GetdarkCube)))
      (Private|StartRoll)
      (bind _percent (Timeline|rollTimeline PlayFromStart)
        (:Update
          (Private|Roll _percent))
        (:Finished
          (Private|EndRoll))))))

(event Input|ActionEvents|InputActionToggleUI
  (params (Key :type Key%20Structure))
  ;[1 1 1] Toggle the UI
  (:Pressed
    (bind _mygamemode (Helper|GetMyGameMode))
    (if (not (Variables|/Game/Blueprints/Game/MyGameMode.MyGameMode_C|GetgameOver _mygamemode))
      (Utilities|FlowControl|FlipFlop
        (:A
          (Public|ResumeMovement))
        (:B
          (Public|PauseMovement))))))

(fn ConstructionScript)

(fn Roll
  (params (progress :type Float%20%28single-precision%29))
  (bind _returnvalue (* progress 9e+01))
  (bind _darkcube (Variables|Default|GetdarkCube))
  (bind _darkcube_2 (Variables|Default|GetdarkCube))
  (bind _moveeast (Variables|/Game/Blueprints/Game/Cubes/DarkCube.DarkCube_C|GetmoveEast _darkcube))
  (bind _movenorth (Variables|/Game/Blueprints/Game/Cubes/DarkCube.DarkCube_C|GetmoveNorth _darkcube))
  (bind _returnvalue_2 (Math|Conversions|ToFloat(Integer) _movenorth))
  (bind _returnvalue_3 (Math|Conversions|ToFloat(Integer) _moveeast))
  (bind _returnvalue_4 (* -1 _returnvalue_3))
  (bind _returnvalue_5 (Math|Vector|MakeVector _returnvalue_4 _returnvalue_2 0.0))
  (bind _rotationvector (Default|CalculateRollVector (Variables|Default|GetdarkCube)))
  (bind _pivot (Default|CalculateRollPivot _darkcube_2))
  (Transformation|SetActorLocationAndRotation _darkcube_2 (+ _pivot (Math|Vector|RotateVectorAroundAxis _rotationvector _returnvalue _returnvalue_5)) (Math|Rotator|CombineRotators (Variables|/Game/Blueprints/Game/Cubes/DarkCube.DarkCube_C|GetlastRotation _darkcube_2) (Math|Vector|RotatorfromAxisandAngle _returnvalue_5 _returnvalue))))

(fn StartRoll
  (bind _darkcube (Variables|Default|GetdarkCube))
  ;[1 1 1] Increment Time
  (bind _mygamemode (Helper|GetMyGameMode))
  (Default|IncrementTime _mygamemode)
  ;[1 1 1] Execute "On Releasing" of underlying cube
  (bind _underlayingcube (Private|FindUnderlayingCube))
  (bind _asaction_cube (Utilities|Casting|CastToActionCube _underlayingcube)
    (:then
      (Default|OnReleasing _asaction_cube))
    (:CastFailed
      _))
  ;[1 1 1] Set states
  (Variables|/Game/Blueprints/Game/Cubes/DarkCube.DarkCube_C|SetisRolling _darkcube true)
  (Default|SetState _darkcube (Variables|Default|Getnorth) (Variables|Default|Geteast)))

(fn EndRoll
  (Default|RestoreState (Variables|Default|GetdarkCube))
  (bind _underlayingcube (Private|FindUnderlayingCube))
  (bind _ascube (Utilities|Casting|CastToCube _underlayingcube)
    (:then
      (bind _asaction_cube (Utilities|Casting|CastToActionCube _ascube)
        (:then
          (Default|OnOverlying _asaction_cube))
        (:CastFailed
          _))
      (Variables|Default|Setnorth 0)
      (Variables|Default|Seteast 0)
      (Variables|/Game/Blueprints/Game/Cubes/DarkCube.DarkCube_C|SetisRolling (Variables|Default|GetdarkCube) false))
    (:CastFailed
      (bind _mygamemode (Helper|GetMyGameMode))
      (Default|Failed _mygamemode))))

(fn FindUnderlayingCube
  (bind _darkcube (Variables|Default|GetdarkCube))
  (bind _returnvalue (Transformation|GetActorLocation _darkcube))
  (bind _outactors (Actor|GetAllActorswithInterface "/Game/Blueprints/Game/Cubes/Cube.Cube_C"))
  (for _array_element _outactors
    (if (and (Math|Float|NearlyEqual(Float) (.x (Transformation|GetActorLocation _array_element)) (.x _returnvalue) 1e+01) (Math|Float|NearlyEqual(Float) (.y (Transformation|GetActorLocation _array_element)) (.y _returnvalue) 1e+01))
      (return _array_element))))

(fn ResumeMovement
  (Variables|Default|SetbShowMouseCursor false)
  (Input|ResetIgnoreLookInput)
  (Input|ResetIgnoreMoveInput)
  (Input|SetInputModeGameOnly self))

(fn PauseMovement
  (Variables|Default|SetbShowMouseCursor true)
  (Input|SetIgnoreLookInput true)
  (Input|SetIgnoreMoveInput true)
  (Input|SetInputModeGameandUI self 0 "DoNotLock" false))

(fn GetMyGameMode
  (bind _asmy_game_mode (Utilities|Casting|CastToMyGameMode (Game|GetGameMode)))
  (return _asmy_game_mode))

(fn GetMyHUD
  (bind _asmy_hud (Utilities|Casting|CastToMyHUD (HUD|GetHUD)))
  (return _asmy_hud))

(fn SetDarkCube
  (bind _mygamemode (Helper|GetMyGameMode))
  (bind _output_get (Variables|Default|SetdarkCube (Variables|/Game/Blueprints/Game/MyGameMode.MyGameMode_C|GetdarkCube _mygamemode)))
  (return _output_get))